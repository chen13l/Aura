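; Arcane Shards gameplay ability that shows a targeting magic circle, then casts a series of shard cues around the chosen ground point.
; On input press, it takes the point under the mouse and spawns a BP_PointCollection there to supply randomly rotated ground points.
; A montage event starts a looping timer that fires one GameplayCue per point, then destroys the collection and ends the ability.
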(event Custom|Spawn%20Shards
  (if (< (Variables|Default|GetCount) (Utilities|Array|Length (Variables|Default|GetGroundPoints)))
    (if (< (Variables|Default|GetCount) (Variables|Default|GetNumPoints))
      (Variables|Default|SetSpawnShardsLocation (Transformation|GetWorldLocation (Utilities|Array|Get(acopy) (Variables|Default|GetGroundPoints) (Variables|Default|GetCount))))
      (Math|Integer|IncrementInt (Variables|Default|GetCount)
        (:%20%20
          (Class|GameplayAbility|ExecuteGameplayCuewithParams "(TagName=\"GameplayCue.ArcaneShards\")" (Ability|GameplayCue|MakeGameplayCueParameters :Location (Variables|Default|GetSpawnShardsLocation)))))
      (else
        (Utilities|Time|ClearandInvalidateTimerbyHandle (Variables|Default|GetTimerHandle) :!label _label)
        (Actor|DestroyActor (Variables|Default|GetPointCollection))
        (Ability|EndAbility)))
    (else
      (goto _label))))

(event Ability|EventActivateAbility
  (Utilities|FlowControl|Sequence
    (:then_0
      (Class|PlayerInterface|ShowMagicCircle(Message) (Ability|GetAvatarActorfromActorInfo) 0))
    (:then_1
      (Ability|Tasks|WaitInputPress false
        (:OnPress
          (bind _data (|TargetDataUnderMouse)
            (:TargetDataDelegate
              (bind _returnvalue (Game|SpawnActorfromClass "/Game/Blueprints/AbilitySystem/Aura/Abilities/Arcane/ArcaneShards/BP_PointCollection.BP_PointCollection_C" (Math|Transform|MakeTransform (.ImpactPoint (Collision|BreakHitResult (Ability|TargetData|GetHitResultfromTargetData _data))) "0, 0, 0" "1.000000,1.000000,1.000000") "Undefined" "MultiplyWithRoot" 0 0))
              (Variables|Default|SetPointCollection _returnvalue)
              (Variables|Default|SetGroundPoints (Class|PointCollection|GetGroundPoints _returnvalue (.ImpactPoint (Collision|BreakHitResult (Ability|TargetData|GetHitResultfromTargetData _data))) (Variables|Default|GetNumPoints) (Math|Random|RandomFloatinRange 0.0 3.6e+02)))
              (Class|CombatInterface|SetFacingTarget(Message) (Ability|GetAvatarActorfromActorInfo) (Variables|Default|GetSpawnShardsLocation))
              (|PlayMontageandWaitProxy "None" "/Game/Assets/Characters/Aura/Animations/Abilities/AM_Cast_ArcaneShards.AM_Cast_ArcaneShards" 1.0 "None" false 1.0 0.0
                (:then
                  (Ability|Tasks|WaitGameplayEvent "(TagName=\"Event.Montage.ArcaneShards\")" 0 true
                    (:EventReceived
                      (bind _returnvalue_2 (Utilities|Time|SetTimerbyEvent (delegate Custom|Spawn%20Shards) (Variables|Default|GetSpawnDeltaTime) true))
                      (Variables|Default|SetTimerHandle _returnvalue_2)
                      (CallFunction|SpawnShards)
                      (Class|PlayerInterface|HideMagicCircle(Message) (Ability|GetAvatarActorfromActorInfo)))))))))))))

(event Ability|EventOnEndAbility
  (params (bWasCancelled :type Boolean)))