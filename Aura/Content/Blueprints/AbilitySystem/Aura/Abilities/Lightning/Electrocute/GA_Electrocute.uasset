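; Electrocute gameplay ability: a channeled lightning beam at the target under the mouse that chains to additional targets.
; A montage event locks movement, adds ShockLoop gameplay cues and starts a looping timer that commits cost and applies lightning damage.
; Input release after a minimum time, failed cost or primary target death stops it, restoring movement, removing cues and committing cooldown.
; On ending, the server also applies a damage effect to each target.
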(event Custom|DamageAndCostEvent
  (bind _returnvalue (Ability|CommitAbilityCost false))
  (if _returnvalue
    (CallFunction|ApplyDamage)
    (else
      (CallFunction|ClearTimerandAbility))))

(event Ability|EventActivateAbility
  (CallFunction|CheckCombatInterface)
  (bind _data (|TargetDataUnderMouse)
    (:TargetDataDelegate
      (bind _output_get (Variables|Default|SetMouseHitResult (Ability|TargetData|GetHitResultfromTargetData _data)))
      (Class|AuraBeamSpell|SetTargetDataInfo _output_get)
      (Class|AuraBeamSpell|SetOwnerParams)
      (Utilities|FlowControl|Sequence
        (:then_0
          (Variables|/Script/Engine.PlayerController|SetbShowMouseCursor (Variables|Default|GetOwnerPlayerController) false)
          (Class|CombatInterface|SetFacingTarget(Message) (Ability|GetAvatarActorfromActorInfo) (Variables|Default|GetMouseHitLocation))
          (GameplayCue|ExecuteGameplayCue :GameplayCueTag "(TagName=\"GameplayCue.Electrocute\")")
          (|PlayMontageandWaitProxy "None" (Variables|Default|GetMontage_Electrocute) 1.0 "None" false 1.0 0.0
            (:then
              (Ability|Tasks|WaitGameplayEvent "(TagName=\"Event.Montage.Electrocute\")" 0 true
                (:EventReceived
                  (CallFunction|InShockLoop)
                  (CallFunction|SpawnBeam)
                  (bind _returnvalue (Utilities|Time|SetTimerbyEvent (delegate Custom|DamageAndCostEvent) (Variables|Default|GetDamageDeltaTime) true))
                  (Variables|Default|SetDamageAndCostTimerHandle _returnvalue))))))
        (:then_1
          (bind _timeheld (Ability|Tasks|WaitInputRelease false)
            (:OnRelease
              (bind _output_get_2 (Variables|Default|SetTimeHeld _timeheld))
              (if (< _output_get_2 (Variables|Default|GetMinSpellTime))
                (Utilities|FlowControl|Delay (- (Variables|Default|GetMinSpellTime) (Variables|Default|GetTimeHeld))))
              (CallFunction|ClearTimerandAbility))))))))

(event EventPrimaryTargetDie
  (params (TargetActor :type Actor%20Object%20Reference))
  (GameplayCue|RemoveGameplayCueOnActor(Looping) TargetActor "(TagName=\"GameplayCue.ShockLoop\")" (Variables|Default|GetFirstTargetCueParams))
  (Ability|CommitAbilityCooldown false)
  (CallFunction|ClearTimerandAbility))

(event EventAdditionalTargetDie
  (params (TargetActor :type Actor%20Object%20Reference))
  (CallFunction|RemoveCueFormAdditionalTarget TargetActor)
  (Utilities|Map|Remove (Variables|Default|GetActorToCueParamsMap) TargetActor))

(fn CheckCombatInterface
  (if (not (Utilities|DoesObjectImplementInterface (Ability|GetAvatarActorfromActorInfo) "/Script/Aura.CombatInterface"))
    (Ability|EndAbility)))

(fn PrepareEnding
  (bind _mousehitactor (Variables|Default|GetMouseHitActor))
  (Variables|/Script/Engine.PlayerController|SetbShowMouseCursor (Variables|Default|GetOwnerPlayerController) true)
  (Class|CombatInterface|SetinShockLoop(Message) (Ability|GetAvatarActorfromActorInfo) false)
  (Pawn|Components|CharacterMovement|SetMovementMode (Variables|/Script/Engine.Character|GetCharacterMovement (Variables|Default|GetOwnerCharacter)) "MOVE_Walking" 0)
  (if (Variables|Default|GetFirstTargetImplementInterface)
    (GameplayCue|RemoveGameplayCueOnActor(Looping) _mousehitactor "(TagName=\"GameplayCue.ShockLoop\")" (Variables|Default|GetFirstTargetCueParams))
    (Ability|HasAuthority
      (:True
        (Class|AuraAbilitySystemLibrary|ApplyDamageEffect (Class|AuraDamageGameplayAbility|MakeAuraDamageEffectParams _mousehitactor)))
      (:False
        _))
    (for _array_element (Variables|Default|GetAdditionalTargets)
      (CallFunction|RemoveCueFormAdditionalTarget _array_element)
      (Ability|HasAuthority
        (:True
          (Class|AuraAbilitySystemLibrary|ApplyDamageEffect (Class|AuraDamageGameplayAbility|MakeAuraDamageEffectParams _array_element)))))
    (else
      (GameplayCue|RemoveGameplayCueOnActor(Looping) (Ability|GetAvatarActorfromActorInfo) "(TagName=\"GameplayCue.ShockLoop\")" (Variables|Default|GetFirstTargetCueParams)))))

(fn InShockLoop
  (Class|CombatInterface|SetinShockLoop(Message) (Ability|GetAvatarActorfromActorInfo) true)
  (Pawn|Components|CharacterMovement|DisableMovement (Variables|/Script/Engine.Character|GetCharacterMovement (Variables|Default|GetOwnerCharacter))))

(fn SpawnBeam
  (bind _mousehitactor (Variables|Default|GetMouseHitActor))
  (bind _returnvalue (Utilities|DoesObjectImplementInterface _mousehitactor "/Script/Aura.CombatInterface"))
  (Class|AuraBeamSpell|TraceFirstTarget (Variables|Default|GetMouseHitLocation))
  (bind _returnvalue_2 (Class|CombatInterface|GetWeapon(Message) (Ability|GetAvatarActorfromActorInfo)))
  (LocalVariables|SetWeapon _returnvalue_2)
  (Variables|Default|SetFirstTargetCueParams (Ability|GameplayCue|MakeGameplayCueParameters :Location (Variables|Default|GetMouseHitLocation) :SourceObject (Variables|Default|GetMouseHitActor) :TargetAttachComponent (LocalVariables|GetWeapon)))
  (Variables|Default|SetFirstTargetImplementInterface _returnvalue)
  (if _returnvalue
    (LocalVariables|SetCueTarget (Variables|Default|GetMouseHitActor))
    (else
      (LocalVariables|SetCueTarget (Ability|GetAvatarActorfromActorInfo))))
  (GameplayCue|AddGameplayCueOnActor(Looping) (LocalVariables|GetCueTarget) "(TagName=\"GameplayCue.ShockLoop\")" (Variables|Default|GetFirstTargetCueParams))
  (if (Variables|Default|GetFirstTargetImplementInterface)
    (bind _outadditionaltargets (Class|AuraBeamSpell|StoreAdditionalTarget))
    (bind _output_get (Variables|Default|SetAdditionalTargets _outadditionaltargets))
    (for _array_element _output_get
      (CallFunction|AddShockLoopCuetoAdditionalTargets _array_element))))

(fn AddShockLoopCuetoAdditionalTargets
  (params (AdditionalTarget :type Actor%20Object%20Reference))
  (bind _output_get (LocalVariables|SetTarget AdditionalTarget))
  (Utilities|Map|Add (Variables|Default|GetActorToCueParamsMap) _output_get (Ability|GameplayCue|MakeGameplayCueParameters :Location (Transformation|GetActorLocation (LocalVariables|GetTarget)) :SourceObject (LocalVariables|GetTarget) :TargetAttachComponent (Variables|/Script/Engine.Actor|GetRootComponent (Variables|Default|GetMouseHitActor))))
  (GameplayCue|AddGameplayCueOnActor(Looping) (LocalVariables|GetTarget) "(TagName=\"GameplayCue.ShockLoop\")" (Ability|GameplayCue|MakeGameplayCueParameters :Location (Transformation|GetActorLocation (LocalVariables|GetTarget)) :SourceObject (LocalVariables|GetTarget) :TargetAttachComponent (Variables|/Script/Engine.Actor|GetRootComponent (Variables|Default|GetMouseHitActor)))))

(fn ApplyDamage
  (CallFunction|ApplyDamageSingleTarget (Variables|Default|GetMouseHitActor))
  (for _array_element (Variables|Default|GetAdditionalTargets)
    (CallFunction|ApplyDamageSingleTarget _array_element)))

(fn ApplyDamageSingleTarget
  (params (Actor :type Actor%20Object%20Reference))
  (bind _returnvalue (Ability|GetAbilitySystemComponentfromActorInfo))
  (bind _returnvalue_2 (Ability|GetAbilitySystemComponent Actor))
  (bind _returnvalue_3 (Ability|GameplayEffect|AssignTagSetbyCallerMagnitude (GameplayEffects|MakeOutgoingSpec _returnvalue (Variables|Default|GetDamageEffectClass) (Math|Conversions|ToFloat(Integer) (Ability|GetAbilityLevel)) (GameplayEffects|MakeEffectContext _returnvalue)) "(TagName=\"Damage.Lightning\")" (Class|AuraDamageGameplayAbility|GetDamageatLevel)))
  (Utilities|IsValid _returnvalue_2
    (:Is%20Valid
      (GameplayEffects|ApplyGameplayEffectSpecToSelf _returnvalue_2 _returnvalue_3))))

(fn ClearTimerandAbility
  (bind _damageandcosttimerhandle (Variables|Default|GetDamageAndCostTimerHandle))
  (if (Utilities|Time|IsValidTimerHandle _damageandcosttimerhandle)
    (Utilities|Time|ClearandInvalidateTimerbyHandle _damageandcosttimerhandle))
  (CallFunction|PrepareEnding)
  (Ability|CommitAbilityCooldown false)
  (Utilities|Map|Clear (Variables|Default|GetActorToCueParamsMap))
  (Utilities|Array|Clear (Variables|Default|GetAdditionalTargets))
  (Variables|Default|SetMouseHitActor 0)
  (Variables|Default|SetFirstTargetImplementInterface false)
  (Variables|Default|SetTimeHeld 0.0)
  (Ability|EndAbility))

(fn RemoveCueFormAdditionalTarget
  (params (InputPin :type Actor%20Object%20Reference))
  (bind _actortocueparamsmap (Variables|Default|GetActorToCueParamsMap))
  (bind (_value _returnvalue) (Utilities|Map|Find _actortocueparamsmap InputPin))
  (if _returnvalue
    (GameplayCue|RemoveGameplayCueOnActor(Looping) InputPin "(TagName=\"GameplayCue.ShockLoop\")" _value)))