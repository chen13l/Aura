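; GA_Electrocute is Aura's channeled lightning ability, holding a shock beam at the point under the mouse until input is released.
; Activation captures mouse target data, turns the avatar and plays a montage whose gameplay event locks movement and spawns the beam.
; The beam is a ShockLoop gameplay cue attached to the weapon, placed on the hit combat actor or otherwise the caster.
; Release removes that cue, restores cursor and walking, and ends the ability.
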(event Ability|EventActivateAbility
  (CallFunction|CheckCombatInterface)
  (bind _data (|TargetDataUnderMouse)
    (:TargetDataDelegate
      (bind _output_get (Variables|Default|SetMouseHitResult (Ability|TargetData|GetHitResultfromTargetData _data)))
      (Class|AuraBeamSpell|SetTargetDataInfo _output_get)
      (Class|AuraBeamSpell|SetOwnerParams)
      (Utilities|FlowControl|Sequence
        (:then_0
          (Variables|/Script/Engine.PlayerController|SetbShowMouseCursor (Variables|Default|GetOwnerPlayerController) false)
          (Class|CombatInterface|SetFacingTarget(Message) (Ability|GetAvatarActorfromActorInfo) (Variables|Default|GetMouseHitLocation))
          (GameplayCue|ExecuteGameplayCue :GameplayCueTag "(TagName=\"GameplayCue.Electrocute\")")
          (|PlayMontageandWaitProxy "None" (Variables|Default|GetMontage_Electrocute) 1.0 "None" false 1.0 0.0
            (:then
              (Ability|Tasks|WaitGameplayEvent "(TagName=\"Event.Montage.Electrocute\")" 0 true
                (:then
                  (CallFunction|InShockLoop)
                  (CallFunction|SpawnBeam))))))
        (:then_1
          (Ability|Tasks|WaitInputRelease false
            (:OnRelease
              (CallFunction|PrepareEnding)
              (Ability|EndAbility))))))))

(fn CheckCombatInterface
  (if (not (Utilities|DoesObjectImplementInterface (Ability|GetAvatarActorfromActorInfo) "/Script/Aura.CombatInterface"))
    (Ability|EndAbility)))

(fn PrepareEnding
  (Variables|/Script/Engine.PlayerController|SetbShowMouseCursor (Variables|Default|GetOwnerPlayerController) true)
  (Class|CombatInterface|SetinShockLoop(Message) (Ability|GetAvatarActorfromActorInfo) false)
  (Pawn|Components|CharacterMovement|SetMovementMode (Variables|/Script/Engine.Character|GetCharacterMovement (Variables|Default|GetOwnerCharacter)) "MOVE_Walking" 0)
  (if (Variables|Default|GetFirstTargetImplementInterface)
    (GameplayCue|RemoveGameplayCueOnActor(Looping) (Variables|Default|GetMouseHitActor) "(TagName=\"GameplayCue.ShockLoop\")" (Variables|Default|GetFirstTargetCueParams))
    (else
      (GameplayCue|RemoveGameplayCueOnActor(Looping) (Ability|GetAvatarActorfromActorInfo) "(TagName=\"GameplayCue.ShockLoop\")" (Variables|Default|GetFirstTargetCueParams))))
  (bind _outadditionaltargets (Class|AuraBeamSpell|StoreAdditionalTarget))
  (for _array_element _outadditionaltargets
    _))

(fn InShockLoop
  (Class|CombatInterface|SetinShockLoop(Message) (Ability|GetAvatarActorfromActorInfo) true)
  (Pawn|Components|CharacterMovement|DisableMovement (Variables|/Script/Engine.Character|GetCharacterMovement (Variables|Default|GetOwnerCharacter))))

(fn SpawnBeam
  (bind _mousehitactor (Variables|Default|GetMouseHitActor))
  (bind _returnvalue (Utilities|DoesObjectImplementInterface _mousehitactor "/Script/Aura.CombatInterface"))
  (Class|AuraBeamSpell|TraceFirstTarget (Variables|Default|GetMouseHitLocation))
  (bind _returnvalue_2 (Class|CombatInterface|GetWeapon(Message) (Ability|GetAvatarActorfromActorInfo)))
  (LocalVariables|SetWeapon _returnvalue_2)
  (Variables|Default|SetFirstTargetCueParams (Ability|GameplayCue|MakeGameplayCueParameters :Location (Variables|Default|GetMouseHitLocation) :SourceObject (Variables|Default|GetMouseHitActor) :TargetAttachComponent (LocalVariables|GetWeapon)))
  (Variables|Default|SetFirstTargetImplementInterface _returnvalue)
  (if _returnvalue
    (LocalVariables|SetCueTarget (Variables|Default|GetMouseHitActor))
    (else
      (LocalVariables|SetCueTarget (Ability|GetAvatarActorfromActorInfo))))
  (GameplayCue|AddGameplayCueOnActor(Looping) (LocalVariables|GetCueTarget) "(TagName=\"GameplayCue.ShockLoop\")" (Variables|Default|GetFirstTargetCueParams)))