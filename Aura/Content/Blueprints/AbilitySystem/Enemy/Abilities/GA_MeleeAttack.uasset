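; GA_MeleeAttack is an enemy gameplay ability that performs a melee attack on the avatar's current combat target.
; It faces the target, plays a random tagged attack montage, and waits for that montage's gameplay event.
; On the event, it finds live players within a radius of the montage's combat socket and damages non-friendly ones with blood effects.
; Any hit fires the MeleeAttack gameplay cue, passing the montage tag and impact location.
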(event Ability|EventActivateAbility
  (bind _returnvalue (Ability|GetAvatarActorfromActorInfo))
  (bind _returnvalue_2 (Ability|GetAvatarActorfromActorInfo))
  (bind _returnvalue_3 (Ability|GetAvatarActorfromActorInfo))
  (Variables|Default|SetHasHitTarget false)
  (bind _ascombat_interface (Utilities|Casting|CastToCombatInterface _returnvalue))
  (bind _returnvalue_4 (Class|EnemyInterface|GetCombatTarget(Message) _returnvalue))
  (Utilities|IsValid _returnvalue_4
    (:Is%20Valid
      (Class|CombatInterface|SetFacingTarget _ascombat_interface (Transformation|GetActorLocation _returnvalue_4))
      (bind _returnvalue_5 (Class|CombatInterface|GetAttackMontages(Message) (Ability|GetAvatarActorfromActorInfo)))
      (Variables|Default|SetTaggedMontage (Class|AuraDamageGameplayAbility|GetRandomAttackMontage _returnvalue_5))
      (|PlayMontageandWaitProxy "None" (.Montage (Utilities|Struct|BreakTaggedMontage (Variables|Default|GetTaggedMontage))) 1.0 "None" false 1.0 0.0
        (:then
          (Ability|Tasks|WaitGameplayEvent (.MontageTag (Utilities|Struct|BreakTaggedMontage (Variables|Default|GetTaggedMontage))) 0
            (:EventReceived
              (bind _returnvalue_6 (Class|CombatInterface|GetCombatSocketLocation(Message) (Ability|GetAvatarActorfromActorInfo) (.SocketTag (Utilities|Struct|BreakTaggedMontage (Variables|Default|GetTaggedMontage)))))
              (bind _output_get (Variables|Default|SetCombatSocketLocation _returnvalue_6))
              (bind _outoverlappingactors (Class|AuraAbilitySystemLibrary|GetLivePlayerWithinRadius _returnvalue_2 (Utilities|Array|MakeArray _returnvalue_2) (Variables|Default|GetRadius) _output_get))
              (for _array_element _outoverlappingactors
                (if (Class|AuraAbilitySystemLibrary|IsNotFriendly _returnvalue_2 _array_element)
                  (Class|AuraDamageGameplayAbility|CauseDamage _array_element)
                  (Variables|Default|SetHasHitTarget true)
                  (Class|CombatInterface|GetBloodEffect(Message) _array_element)
                  (else
                    (Ability|EndAbility))))
              (if (Variables|Default|GetHasHitTarget)
                (bind _returnvalue_7 (Class|EnemyInterface|GetCombatTarget(Message) _returnvalue_3))
                (Class|GameplayAbility|ExecuteGameplayCuewithParams "(TagName=\"GameplayCue.MeleeAttack\")" (Ability|GameplayCue|MakeGameplayCueParameters :AggregatedSourceTags (GameplayTags|MakeGameplayTagContainerfromTag (.MontageTag (Utilities|Struct|BreakTaggedMontage (Variables|Default|GetTaggedMontage)))) :Location (Variables|Default|GetCombatSocketLocation) :EffectCauser _returnvalue_3 :SourceObject _returnvalue_7)))
              (Ability|EndAbility))))
        (:OnCompleted
          (Ability|EndAbility :!label _label))
        (:OnInterrupted
          (goto _label))
        (:OnCancelled
          (goto _label))))))

(event Ability|EventOnEndAbility
  (params (bWasCancelled :type Boolean)))