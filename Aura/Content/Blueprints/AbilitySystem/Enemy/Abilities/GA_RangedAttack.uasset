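; Enemy ranged attack gameplay ability that fires a projectile at the avatar's combat target.
; On activation it gets a valid target through avatar messages, turns to face it and plays a random tagged attack montage.
; The montage's gameplay event triggers the projectile spawn from the tagged socket toward the target's current location.
; The ability ends shortly after the spawn, or when the montage is interrupted or cancelled.
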(event Ability|EventActivateAbility
  (bind _returnvalue (Ability|GetAvatarActorfromActorInfo))
  (bind _returnvalue_2 (Class|EnemyInterface|GetCombatTarget(Message) _returnvalue))
  (Utilities|IsValid _returnvalue_2
    (:Is%20Valid
      (Class|CombatInterface|SetFacingTarget(Message) _returnvalue (Transformation|GetActorLocation _returnvalue_2))
      (bind _returnvalue_3 (Class|CombatInterface|GetAttackMontages(Message) _returnvalue))
      (Variables|Default|SetTaggedMontage (Class|AuraDamageGameplayAbility|GetRandomAttackMontage _returnvalue_3))
      (|PlayMontageandWaitProxy "None" (.Montage (Utilities|Struct|BreakTaggedMontage (Variables|Default|GetTaggedMontage))) 1.0 "None" false 1.0 0.0
        (:then
          (Ability|Tasks|WaitGameplayEvent (.MontageTag (Utilities|Struct|BreakTaggedMontage (Variables|Default|GetTaggedMontage))) 0 true
            (:EventReceived
              (bind _returnvalue_4 (Class|EnemyInterface|GetCombatTarget(Message) (Ability|GetAvatarActorfromActorInfo)))
              (Class|AuraProjectileSpell|SpawnProjectile (Transformation|GetActorLocation _returnvalue_4) (.SocketTag (Utilities|Struct|BreakTaggedMontage (Variables|Default|GetTaggedMontage))) false 0.0)
              (Utilities|FlowControl|Delay 0.5)
              (Ability|EndAbility))))
        (:OnInterrupted
          (Ability|EndAbility :!label _label))
        (:OnCancelled
          (goto _label))))))

(event Ability|EventOnEndAbility
  (params (bWasCancelled :type Boolean)))