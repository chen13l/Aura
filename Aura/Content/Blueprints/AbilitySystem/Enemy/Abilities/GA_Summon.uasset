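; Enemy gameplay ability that lets a shaman summon random minions at a set of spawn locations.
; It shuffles the locations, plays the summon montage and waits for its gameplay event tag.
; On that event, a loop fires a summon gameplay cue and spawns an AI-possessed minion at each location, facing away from the summoner.
; Each spawn increments the summoner's minion count, and the ability ends once all locations are used.
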(event Ability|EventActivateAbility
  (bind _returnvalue (Class|AuraShamanAbility|GetSpawnLocations))
  (bind _output_get (Variables|Default|SetSpawnLocations _returnvalue))
  (Utilities|Array|Shuffle _output_get)
  (|PlayMontageandWaitProxy "None" "/Game/Assets/Enemies/Shaman/Animations/AM_Shaman_Summon.AM_Shaman_Summon" 1.0 "None" false 1.0 0.0
    (:then
      (Ability|Tasks|WaitGameplayEvent "(TagName=\"Montage.Attack.2\")" 0 true
        (:EventReceived
          (if (< (Variables|Default|GetLocationsIndex) (Utilities|Array|Length (Variables|Default|GetSpawnLocations))) :!label _label
            (Variables|Default|SetChosenLocation (Utilities|Array|Get(acopy) (Variables|Default|GetSpawnLocations) (Variables|Default|GetLocationsIndex)))
            (Class|GameplayAbility|ExecuteGameplayCuewithParams "(TagName=\"GameplayCue.Summon\")" (Ability|GameplayCue|MakeGameplayCueParameters :Location (Variables|Default|GetChosenLocation) :EffectCauser (Ability|GetAvatarActorfromActorInfo)))
            (bind _returnvalue_2 (Game|SpawnActorfromClass (Class|AuraShamanAbility|GetRandomMinionClass) (Math|Transform|MakeTransform (+ (Variables|Default|GetChosenLocation) "0.000000,0.000000,70.000000") (Math|Rotator|FindLookatRotation (Transformation|GetActorLocation (Ability|GetAvatarActorfromActorInfo)) (+ (Variables|Default|GetChosenLocation) "0.000000,0.000000,70.000000")) "1.000000,1.000000,1.000000") "AlwaysSpawn" "MultiplyWithRoot" 0 0))
            (Pawn|SpawnDefaultController _returnvalue_2)
            (Math|Integer|IncrementInt (Variables|Default|GetLocationsIndex)
              (:%20%20
                (Class|CombatInterface|IncrementMinionCount(Message) (Ability|GetAvatarActorfromActorInfo) 1)
                (goto _label)))
            (else
              (Ability|EndAbility))))))))

(event Ability|EventOnEndAbility
  (params (bWasCancelled :type Boolean)))