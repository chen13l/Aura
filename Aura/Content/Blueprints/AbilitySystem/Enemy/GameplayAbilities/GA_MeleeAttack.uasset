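; Enemy melee attack ability that turns the avatar toward its combat target and plays a random tagged attack montage.
; The montage's gameplay event triggers a radius query for live players at the tag's combat socket, damaging those that are not friendly.
; The ability ends after that loop, on hitting a friendly actor, or when the montage completes, is interrupted or is cancelled.
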(event Ability|EventActivateAbility
  (bind _returnvalue (Ability|GetAvatarActorfromActorInfo))
  (bind _returnvalue_2 (Ability|GetAvatarActorfromActorInfo))
  (bind _ascombat_interface (Utilities|Casting|CastToCombatInterface _returnvalue))
  (bind _returnvalue_3 (Class|EnemyInterface|GetCombatTarget(Message) _returnvalue))
  (Utilities|IsValid _returnvalue_3
    (:Is%20Valid
      (Class|CombatInterface|SetFacingTarget _ascombat_interface (Transformation|GetActorLocation _returnvalue_3))
      (bind _returnvalue_4 (Class|CombatInterface|GetAttackMontages(Message) (Ability|GetAvatarActorfromActorInfo)))
      (Variables|Default|SetTaggedMontage (Class|AuraDamageGameplayAbility|GetRandomAttackMontage _returnvalue_4))
      (|PlayMontageandWaitProxy "None" (.Montage (Utilities|Struct|BreakTaggedMontage (Variables|Default|GetTaggedMontage))) 1.0 "None" false 1.0 0.0
        (:then
          (Ability|Tasks|WaitGameplayEvent (.MontageTag (Utilities|Struct|BreakTaggedMontage (Variables|Default|GetTaggedMontage))) 0
            (:EventReceived
              (bind _returnvalue_5 (Class|CombatInterface|GetCombatSocketLocation(Message) (Ability|GetAvatarActorfromActorInfo) (.MontageTag (Utilities|Struct|BreakTaggedMontage (Variables|Default|GetTaggedMontage)))))
              (bind _outoverlappingactors (Class|AuraAbilitySystemLibrary|GetLivePlayerWithinRadius _returnvalue_2 (Utilities|Array|MakeArray _returnvalue_2) (Variables|Default|GetRadius) _returnvalue_5))
              (for _array_element _outoverlappingactors
                (if (Class|AuraAbilitySystemLibrary|IsNotFriendly _returnvalue_2 _array_element)
                  (Class|AuraDamageGameplayAbility|CauseDamage _array_element)
                  (else
                    (Ability|EndAbility))))
              (Ability|EndAbility))))
        (:OnCompleted
          (Ability|EndAbility :!label _label))
        (:OnInterrupted
          (goto _label))
        (:OnCancelled
          (goto _label))))))

(event Ability|EventOnEndAbility
  (params (bWasCancelled :type Boolean)))