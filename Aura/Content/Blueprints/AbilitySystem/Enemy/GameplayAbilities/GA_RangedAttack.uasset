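; Enemy ranged attack gameplay ability that fires a projectile at the avatar's current combat target.
; With a valid target, it turns the avatar to face it and plays a random tagged attack montage.
; It starts a wait for the montage tag's gameplay event, with SpawnProjectile wired to that task's `then` pin, aimed at the target's location.
; Only montage interruption or cancellation explicitly ends the ability.
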(event Ability|EventActivateAbility
  (bind _returnvalue (Ability|GetAvatarActorfromActorInfo))
  (bind _returnvalue_2 (Ability|GetAvatarActorfromActorInfo))
  (bind _returnvalue_3 (Class|EnemyInterface|GetCombatTarget(Message) _returnvalue))
  (Utilities|IsValid _returnvalue_3
    (:Is%20Valid
      (Class|CombatInterface|SetFacingTarget(Message) _returnvalue (Transformation|GetActorLocation _returnvalue_3))
      (bind _returnvalue_4 (Class|CombatInterface|GetAttackMontages(Message) _returnvalue))
      (Variables|Default|SetTaggedMontage (Class|AuraDamageGameplayAbility|GetRandomAttackMontage _returnvalue_4))
      (|PlayMontageandWaitProxy "None" (.Montage (Utilities|Struct|BreakTaggedMontage (Variables|Default|GetTaggedMontage))) 1.0 "None" false 1.0 0.0
        (:then
          (Ability|Tasks|WaitGameplayEvent (.MontageTag (Utilities|Struct|BreakTaggedMontage (Variables|Default|GetTaggedMontage))) 0
            (:then
              (Class|CombatInterface|GetCombatSocketLocation(Message) _returnvalue_2 (.MontageTag (Utilities|Struct|BreakTaggedMontage (Variables|Default|GetTaggedMontage))))
              (bind _returnvalue_5 (Class|EnemyInterface|GetCombatTarget(Message) _returnvalue_2))
              (Class|AuraProjectileSpell|SpawnProjectile (Transformation|GetActorLocation _returnvalue_5)))))
        (:OnInterrupted
          (Ability|EndAbility :!label _label))
        (:OnCancelled
          (goto _label))))))

(event Ability|EventOnEndAbility
  (params (bWasCancelled :type Boolean)))