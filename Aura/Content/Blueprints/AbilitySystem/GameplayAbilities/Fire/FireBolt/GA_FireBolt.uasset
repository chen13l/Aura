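; GA_FireBolt is a gameplay ability that casts a fire bolt projectile at the location under the mouse cursor.
; A target data task supplies the hit location, and the avatar turns toward it through the CombatInterface.
; It plays the cast montage, then spawns the projectile when the Event.Montage.FireBolt gameplay event arrives.
; The ability ends after a short delay following the spawn.
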(event Ability|EventActivateAbility
  (bind _data (|TargetDataUnderMouse)
    (:TargetDataDelegate
      (Variables|Default|SetTargetLocation (.Location (Collision|BreakHitResult (Ability|TargetData|GetHitResultfromTargetData _data))))
      (bind _ascombat_interface (Utilities|Casting|CastToCombatInterface (Ability|GetAvatarActorfromActorInfo)))
      (Class|CombatInterface|SetFacingTarget _ascombat_interface (Variables|Default|GetTargetLocation))
      (|PlayMontageandWaitProxy "None" "/Game/Assets/Characters/Aura/Animations/Abilities/AM_Cast_FireBolt.AM_Cast_FireBolt" 1.0 "None" true 1.0 0.0
        (:then
          (Ability|Tasks|WaitGameplayEvent "(TagName=\"Event.Montage.FireBolt\")" 0
            (:EventReceived
              (Class|AuraProjectileSpell|SpawnProjectile (Variables|Default|GetTargetLocation))
              (Utilities|FlowControl|Delay 1.0)
              (Ability|EndAbility))))))))

(event Ability|EventOnEndAbility
  (params (bWasCancelled :type Boolean)))