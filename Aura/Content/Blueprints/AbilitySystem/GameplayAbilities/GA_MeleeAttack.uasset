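; Melee attack Gameplay Ability that turns the avatar toward its combat target and plays a random attack montage from the combat interface.
; It waits for a montage-tag gameplay event, then damages live players within a radius of the matching combat socket and ends.
; Montage, event tag and socket tag each use a separate random index expression, so they can mismatch.
; Without a valid target, it never calls EndAbility.
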(event Ability|EventActivateAbility
  (bind _returnvalue (Ability|GetAvatarActorfromActorInfo))
  (bind _ascombat_interface (Utilities|Casting|CastToCombatInterface _returnvalue))
  (bind _returnvalue_2 (Class|EnemyInterface|GetCombatTarget(Message) _returnvalue))
  (Utilities|IsValid _returnvalue_2
    (:Is%20Valid
      (Class|CombatInterface|SetFacingTarget _ascombat_interface (Transformation|GetActorLocation _returnvalue_2))
      (bind _returnvalue_3 (Class|CombatInterface|GetAttackMontages(Message) (Ability|GetAvatarActorfromActorInfo)))
      (|PlayMontageandWaitProxy "None" (.Montage (Utilities|Struct|BreakTaggedMontage (Utilities|Array|Get(acopy) _returnvalue_3 (Math|Random|RandomIntegerinRange 0 (- (Utilities|Array|Length _returnvalue_3) 1))))) 1.0 "None" true 1.0 0.0
        (:then
          (Ability|Tasks|WaitGameplayEvent (.MontageTag (Utilities|Struct|BreakTaggedMontage (Utilities|Array|Get(acopy) _returnvalue_3 (Math|Random|RandomIntegerinRange 0 (- (Utilities|Array|Length _returnvalue_3) 1))))) 0
            (:EventReceived
              (bind _returnvalue_4 (Class|CombatInterface|GetCombatSocketLocation(Message) (Ability|GetAvatarActorfromActorInfo) (.MontageTag (Utilities|Struct|BreakTaggedMontage (Utilities|Array|Get(acopy) _returnvalue_3 (Math|Random|RandomIntegerinRange 0 (- (Utilities|Array|Length _returnvalue_3) 1)))))))
              (bind _outoverlappingactors (Class|AuraAbilitySystemLibrary|GetLivePlayerWithinRadius (Ability|GetAvatarActorfromActorInfo) (Variables|Default|GetRadius) _returnvalue_4))
              (for _array_element _outoverlappingactors
                (Class|AuraDamageGameplayAbility|CauseDamage _array_element))
              (Ability|EndAbility))))))))

(event Ability|EventOnEndAbility
  (params (bWasCancelled :type Boolean)))