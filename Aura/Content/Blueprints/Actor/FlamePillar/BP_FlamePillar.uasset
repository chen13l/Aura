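; BP_FlamePillar is a flame pillar actor that animates the brightness of its FireLight.
; From BeginPlay, it randomly picks one of two timelines, and each picks again when it finishes, forming an endless varied loop.
; Timeline updates feed ScaleFlameIntensity, which multiplies the curve value by a base intensity and applies it to the light.
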(event Custom|StartTimeLine_1
  (bind _flameintensity (Timeline|FlameIntensity_1 PlayFromStart)
    (:Update
      (CallFunction|ScaleFlameIntensity _flameintensity))
    (:Finished
      (CallFunction|ChoseTimeLineRandom))))

(event Custom|StartTimeLine_2
  (bind _newtrack_0 (Timeline|FlameIntensity_2 PlayFromStart)
    (:Update
      (CallFunction|ScaleFlameIntensity _newtrack_0))
    (:Finished
      (CallFunction|ChoseTimeLineRandom))))

(event Custom|ChoseTimeLineRandom
  (switch int (Math|Random|RandomIntegerinRange 0 1)
    (:Default
      (CallFunction|StartTimeLine2))
    (:0
      (CallFunction|StartTimeLine1))
    (:1
      (CallFunction|StartTimeLine2))))

(event EventBeginPlay
  (CallFunction|ChoseTimeLineRandom))

(event Collision|EventActorBeginOverlap
  (params (OtherActor :type Actor%20Object%20Reference)))

(event EventTick
  (params (DeltaSeconds :type Float%20%28single-precision%29)))

(fn ConstructionScript)

(fn ScaleFlameIntensity
  (params (Intensity :type Float%20%28double-precision%29))
  (Rendering|Components|Light|SetIntensity (Variables|Default|GetFireLight) (* Intensity (Variables|Default|GetBaseIntensuty))))